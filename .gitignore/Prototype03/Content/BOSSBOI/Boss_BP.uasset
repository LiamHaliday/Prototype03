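; Ice boss character that chases player 0 and starts attacking when close, switching to Phase 2 below half health.
; Tick drives movement and a state machine, with Phase 1 cycling spin, expanding explosion and stomp attacks through Delays.
; Attacks snap sphere or box colliders to a mesh socket, scaling them to detect player overlaps.
; Hits only print debug text, and Phase 2 attacks are stubs that print names or position the box collider.
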(event EventTick
  (params (DeltaSeconds :type Float%20%28single-precision%29))
  (bind _returnvalue (Pawn|GetController))
  (bind _spherical_collider (Variables|Default|GetSpherical%20Collider))
  (Utilities|FlowControl|Sequence
    (:then_0
      (if (Variables|Default|GetIsWalking)
        ;[1 1 1] Move
        (AI|Navigation|SimpleMovetoActor _returnvalue (Game|GetPlayerCharacter 0))
        (if (< (Variables|Default|GetDistanceFromCharacter) 5e+02)
          (Variables|Default|SetAttacking true))
        (else
          ;[1 1 1] Stop Moving
          (AI|Navigation|SimpleMovetoLocation _returnvalue (Transformation|GetActorLocation)))))
    (:then_1
      ;[1 1 1] distance from character
      (bind _output_get (Variables|Default|SetDistanceFromCharacter (Math|Vector|VectorLength (- (Transformation|GetWorldLocation (Variables|/Script/Engine.Actor|GetRootComponent (Game|GetPlayerCharacter 0))) (Transformation|GetWorldLocation (Variables|Collision|GetCapsuleComponent))))))
      (Development|PrintString (Utilities|String|Append "Distance From Character" (Utilities|String|ToString(Float) _output_get)) true true "(R=0.000000,G=0.660000,B=1.000000,A=1.000000)" 0.01))
    (:then_2
      (if (Variables|Default|GetAttacking)
        (switch string (Variables|Default|GetBossState)
          (:Phase%201
            (Development|PrintString "Phase 1" true true "(R=0.000000,G=0.660000,B=1.000000,A=1.000000)" 0.01)
            (switch int (Variables|Default|GetIteratePhase1)
              (:1
                ;[1 1 1] Spin Attack (Uses Spherical Collider)
                (CallFunction|ConnectSocketandCollider "pCube20" (Variables|Default|GeticeBoss_blockout_MESH) (Variables|Default|GetSpherical%20Collider))
                ;;[1 1 1] Init Attack
                (if (Variables|Default|GetInitAttack)
                  (Variables|/Script/Engine.CharacterMovementComponent|SetMaxWalkSpeed (Variables|Character|GetCharacterMovement) 2e+02)
                  (Utilities|FlowControl|Delay 2.0)
                  (Transformation|SetWorldScale3D (Variables|Default|GetSpherical%20Collider) "15.000000,15.000000,15.000000")
                  (Variables|Default|SetInitAttack false)
                  (else
                    ;;[1 1 1] Collision Detection
                    (for _array_element (Collision|GetOverlappingActors (Variables|Default|GetSpherical%20Collider) "/Game/ThirdPersonBP/Blueprints/Player.Player_C" :!class /Script/Engine.PrimitiveComponent)
                      (Utilities|FlowControl|Delay 0.1)
                      (Development|PrintString "Hit Target" true true "(R=0.000000,G=0.660000,B=1.000000,A=1.000000)" 0.5))
                    ;;[1 1 1] Time To Complete attack
                    (Utilities|FlowControl|Delay 1.5)
                    ;;[1 1 1] End Of Attack
                    (Variables|Default|SetIsWalking true)
                    (Variables|Default|SetAttacking false)
                    (Variables|Default|SetInitAttack true)
                    (Transformation|SetWorldScale3D (Variables|Default|GetSpherical%20Collider) "0, 0, 0")
                    (Variables|Default|SetIteratePhase1 2)
                    (Variables|/Script/Engine.CharacterMovementComponent|SetMaxWalkSpeed (Variables|Character|GetCharacterMovement) 5e+02))))
              (:2
                ;[1 1 1] Explosion (Uses Spherical Collider)
                ;;[1 1 1] Can't Walk
                (Variables|Default|SetIsWalking false)
                (CallFunction|ConnectSocketandCollider "pCube20" (Variables|Default|GeticeBoss_blockout_MESH) (Variables|Default|GetSpherical%20Collider))
                ;;[1 1 1] Init Attack
                (if (Variables|Default|GetInitAttack)
                  (Utilities|FlowControl|Delay 2.0)
                  (Variables|Default|SetInitAttack false)
                  (else
                    ;;[1 1 1] Collision Detection
                    (Transformation|SetWorldScale3D _spherical_collider (+ (Transformation|GetWorldScale _spherical_collider) (* (Variables|Default|GetNewVar_0) (Utilities|Time|GetWorldDeltaSeconds))))
                    (for _array_element_2 (Collision|GetOverlappingActors (Variables|Default|GetSpherical%20Collider) "/Game/ThirdPersonBP/Blueprints/Player.Player_C" :!class /Script/Engine.PrimitiveComponent)
                      (Utilities|FlowControl|DoOnce false
                        (:Completed
                          (Development|PrintString "Ouchie"))))
                    (Utilities|FlowControl|Delay 2.0)
                    ;;[1 1 1] End Of Attack
                    (Variables|Default|SetIteratePhase1 3)
                    (Transformation|SetWorldScale3D (Variables|Default|GetSpherical%20Collider) "0, 0, 0")
                    (Variables|Default|SetIsWalking true)
                    (Variables|Default|SetInitAttack true)
                    (Variables|Default|SetAttacking false)
                    (Utilities|FlowControl|DoOnce false) ; enters at Reset
                  )))
              (:3
                ;[1 1 1] Stompy (Uses Box Collider)
                ;;[1 1 1] Can't Walk
                (Variables|Default|SetIsWalking false)
                (CallFunction|ConnectSocketandCollider "pCube20" (Variables|Default|GeticeBoss_blockout_MESH) (Variables|Default|GetBox%20Collider))
                ;;[1 1 1] Init Attack
                (if (Variables|Default|GetInitAttack)
                  (Utilities|FlowControl|Delay 2.0)
                  (Transformation|SetWorldScale3D (Variables|Default|GetBox%20Collider) "8.000000,8.000000,8.000000")
                  (Variables|Default|SetInitAttack false)
                  (else
                    ;;[1 1 1] Collision Detection
                    (for _array_element_3 (Collision|GetOverlappingActors (Variables|Default|GetBox%20Collider) "/Game/ThirdPersonBP/Blueprints/Player.Player_C" :!class /Script/Engine.PrimitiveComponent)
                      (Utilities|FlowControl|DoOnce false
                        (:Completed
                          (Development|PrintString "That Hurt"))))
                    ;;[1 1 1] End Of Attack
                    (Variables|Default|SetIteratePhase1 1)
                    (Variables|Default|SetIsWalking true)
                    (Transformation|SetWorldScale3D (Variables|Default|GetBox%20Collider) "0, 0, 0")
                    (Variables|Default|SetInitAttack true)
                    (Variables|Default|SetIsWalking false)
                    (Utilities|FlowControl|DoOnce false) ; enters at Reset
                  )))
              (:4
                (Development|PrintString "Hello"))))
          (:Phase%202
            (Development|PrintString "Phase 2" true true "(R=0.000000,G=0.660000,B=1.000000,A=1.000000)" 0.01)
            (switch int (Variables|Default|GetIteratePhase2)
              (:1
                (Development|PrintString "Side Swipe Attack" true true "(R=0.000000,G=0.660000,B=1.000000,A=1.000000)" 0.01)
                (CallFunction|ConnectSocketandCollider "pCube20" (Variables|Default|GeticeBoss_blockout_MESH) (Variables|Default|GetBox%20Collider)))
              (:2
                (Development|PrintString "Wall" true true "(R=0.000000,G=0.660000,B=1.000000,A=1.000000)" 0.01))
              (:3
                (Development|PrintString "Tail Swipe" true true "(R=0.000000,G=0.660000,B=1.000000,A=1.000000)" 0.01)
                (CallFunction|ConnectSocketandCollider "pCube20" (Variables|Default|GeticeBoss_blockout_MESH) (Variables|Default|GetBox%20Collider)))
              (:4
                (Development|PrintString "Forward Slashing Combo" true true "(R=0.000000,G=0.660000,B=1.000000,A=1.000000)" 0.01)
                (CallFunction|ConnectSocketandCollider "pCube20" (Variables|Default|GeticeBoss_blockout_MESH) (Variables|Default|GetBox%20Collider))))))))
    (:then_3
      ;[1 1 1] Phase 2 condition
      (if (< (Variables|Default|GetCurrentBossHealth) (/ (Variables|Default|GetMaxBossHealth) 2))
        (Variables|Default|SetBossState "Phase 2")))))

(event EventBeginPlay
  ;[1 1 1] initialisers
  (Variables|Default|SetBossState "Phase 1")
  (Variables|/Script/Engine.CharacterMovementComponent|SetMaxWalkSpeed (Variables|Character|GetCharacterMovement) 5e+02))

(fn ConstructionScript)

(fn ConnectSocketandCollider
  (params (Socket :type Name) (Skeletal%20Object :type Scene%20Component%20Object%20Reference) (Collider :type Scene%20Component%20Object%20Reference))
  (Transformation|SetWorldLocationAndRotation Collider (Transformation|GetSocketLocation Skeletal%20Object Socket) (Transformation|GetSocketRotation Skeletal%20Object Socket) false false))